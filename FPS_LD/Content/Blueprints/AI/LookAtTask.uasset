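; LookAtTask is a behavior tree task that turns a ShooterController's pawn toward the player character.
; On tick it finds the look-at rotation to player 0, keeps only the yaw, and eases the pawn toward it with RInterpTo at RotationSpeed.
; It then finishes successfully at once, so each execution makes one interpolation step and a full turn takes repeated runs.
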(event `self.ReceiveTick`
  (params (OwnerActor :type "Actor Object Reference") (DeltaSeconds :type "Float (single-precision)"))
  (bind _asshooter_controller (cast `/Game/Blueprints/AI/ShooterController` OwnerActor))
  (bind _returnvalue (`Controller.K2_GetPawn` _asshooter_controller))
  (`Actor.SetActorRotation` _returnvalue (`KismetMathLibrary.RInterpTo` (`Actor.K2_GetActorRotation` _returnvalue) (`KismetMathLibrary.MakeRotator` 0.0 0.0 (.yaw (`KismetMathLibrary.FindLookAtRotation` (`Actor.K2_GetActorLocation` _returnvalue) (`Actor.K2_GetActorLocation` (`GameplayStatics.GetPlayerCharacter` 0))))) (`self.DeltaTime`) (`self.rotationSpeed`)))
  (`self.FinishExecute` true))