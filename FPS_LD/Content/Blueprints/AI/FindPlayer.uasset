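; Behavior tree task that detects the player for AI pawns driven by a MeleeController.
; It compares the horizontal distance to player character 0 against the controller's PerceptionRadius, with no line-of-sight check.
; When in range, it writes the player to the Player blackboard key and succeeds.
; Otherwise it fails without clearing the key, as it also does for other controller types.
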(event `self.ReceiveExecute`
  (params (OwnerActor :type "Actor Object Reference"))
  (bind _returnvalue (`GameplayStatics.GetPlayerCharacter` 0))
  (bind _returnvalue_2 (`AIBlueprintHelperLibrary.GetAIController` OwnerActor))
  (bind _asmelee_controller (cast `/Game/Blueprints/AI/MeleeController` _returnvalue_2)
    (:`then`
      (`|ExecutionSequence`
        (:`then_0`
          (bind _returnvalue_3 (<= (`Actor.GetHorizontalDistanceTo` _returnvalue OwnerActor) (`/Game/Blueprints/AI/MeleeController.Perception Radius` _asmelee_controller)))
          (if _returnvalue_3
            (`BTFunctionLibrary.SetBlackboardValueAsObject` (`self.Player`) _returnvalue)))
        (:`then_1`
          (`self.FinishExecute` _returnvalue_3))))
    (:`CastFailed`
      (`self.FinishExecute` false))))