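; AmmoBoxBP is an ammo pickup that refills the player's ammo when its Trigger component is overlapped.
; The overlap handler casts player character 0 to FirstPersonCharacter without checking which actor overlapped.
; If Ammo is below MaxAmmo, it adds AmmoFill, capped at MaxAmmo, and destroys the box.
; At full ammo the box stays in the world.
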(event `self.ReceiveBeginPlay`)

(event `self.Trigger.OnComponentBeginOverlap`
  (params (OtherActor :type "Actor Object Reference") (OtherComp :type "PrimitiveComponent Object Reference") (OtherBodyIndex :type Integer) (bFromSweep :type Boolean) (SweepResult :type "HitResult Structure (by ref)"))
  (bind _ammofill (`self.ammoFill`))
  (bind _asfirst_person_character (cast `/Game/FirstPersonBP/Blueprints/FirstPersonCharacter` (`GameplayStatics.GetPlayerCharacter` 0)))
  (bind _ammo (`/Game/FirstPersonBP/Blueprints/FirstPersonCharacter.Ammo` _asfirst_person_character))
  (bind _maxammo (`/Game/FirstPersonBP/Blueprints/FirstPersonCharacter.MaxAmmo` _asfirst_person_character))
  (if (< _ammo _maxammo)
    (if (<= _ammo (- _maxammo _ammofill))
      (set `/Game/FirstPersonBP/Blueprints/FirstPersonCharacter.Ammo` (+ _ammo _ammofill) _asfirst_person_character)
      (else
        (set `/Game/FirstPersonBP/Blueprints/FirstPersonCharacter.Ammo` _maxammo _asfirst_person_character)))
    (`self.K2_DestroyActor`)))

(event `self.ReceiveActorBeginOverlap`
  (params (OtherActor :type "Actor Object Reference")))

(event `self.ReceiveTick`
  (params (DeltaSeconds :type "Float (single-precision)")))

(fn `UserConstructionScript`)